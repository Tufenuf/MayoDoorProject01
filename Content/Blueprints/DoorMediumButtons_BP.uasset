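; Hallway airlock door that unlocks through a puzzle of four wall buttons shot in order with first-person projectiles.
; Correct hits turn panels green, out-of-order hits reset earlier ones, and hitting the fourth increments the player character's PuzzlesComplete.
; Once solved, TriggerSouth overlap plays two chained timelines that slide the door back, then up with sound.
; Leaving the trigger reverses them after a delay, using DoorOpen to chain the closing stages.
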(event OnComponentEndOverlap(TriggerSouth)
  (params (OverlappedComponent :type Primitive%20Component%20Object%20Reference) (OtherActor :type Actor%20Object%20Reference) (OtherComp :type Primitive%20Component%20Object%20Reference) (OtherBodyIndex :type Integer))
  ;[1 1 1] EndOverlapCheck
  (if (Math|Boolean|ANDBoolean (stale OnComponentHit(HitCheck1) _output_get) (stale OnComponentHit(HitCheck2) _output_get) (stale OnComponentHit(HitCheck3) _output_get) (stale OnComponentHit(HitCheck4) _output_get))
    (Utilities|Casting|CastToFirstPersonCharacter OtherActor)
    (Utilities|FlowControl|Delay 0.5)
    ;[1 1 1] DoorAnimUp
    (bind _dooranimup (Timeline|DoorAnimUp Reverse)
      (:Update
        (Transformation|SetRelativeLocation (Variables|Default|GetHall_Door_L) (Math|Vector|Lerp(Vector) "0,-20.000000, 0" "0,-30.000000,400.000000" _dooranimup) false false))
      (:Finished
        (if (Variables|Default|GetDoorOpen)
          ;[1 1 1] DoorAnimBack
          (bind _dooranimunlock (Timeline|DoorAnimBack Reverse)
            (:Update
              (Transformation|SetRelativeLocation (Variables|Default|GetHall_Door_L) (Math|Vector|Lerp(Vector) "0, 0, 0" "0,-20.000000, 0" _dooranimunlock) false false))
            (:Finished
              (if (Math|Vector|Equal(Vector) (.Location (Math|Transform|BreakTransform (Transformation|GetRelativeTransform (Variables|Default|GetHall_Door_L)))) "0,-20.000000, 0" 1.0)
                (Utilities|FlowControl|Delay 1.0)
                (Audio|PlaySoundatLocation "/Game/Sounds/AirlockDoorOpen.AirlockDoorOpen" "0, 0, 0" "0, 0, 0" 1.0 1.0 0.0 0 0 0)
                (Timeline|DoorAnimUp Play))))
          (else
            (Variables|Default|SetDoorOpen true)))))))

(event OnComponentHit(HitCheck4)
  (params (HitComponent :type Primitive%20Component%20Object%20Reference) (OtherActor :type Actor%20Object%20Reference) (OtherComp :type Primitive%20Component%20Object%20Reference) (NormalImpulse :type Vector :default "0, 0, 0") (Hit :type Hit%20Result%20Structure%20%28by%20ref%29))
  ;[1 1 1] Button Check
  (bind _asfirst_person_projectile (Utilities|Casting|CastToFirstPersonProjectile OtherActor))
  (Actor|DestroyActor _asfirst_person_projectile)
  (if (Math|Boolean|ANDBoolean (Variables|Default|GetButtonCheck1) (Variables|Default|GetButtonCheck2) (Variables|Default|GetButtonCheck3))
    (Rendering|Material|SetMaterial (Variables|Default|GetHall_Wall_C4) 2 "/Game/Mayo_OriginalMaterials/M_GreenLight.M_GreenLight")
    (bind _output_get (Variables|Default|SetButtonCheck4 true))
    ;[1 1 1] IncrementPuzzleScore
    (if (Math|Boolean|ANDBoolean (stale OnComponentHit(HitCheck1) _output_get) (stale OnComponentHit(HitCheck2) _output_get) (stale OnComponentHit(HitCheck3) _output_get) _output_get)
      (bind _asfirst_person_character (Utilities|Casting|CastToFirstPersonCharacter (Game|GetPlayerCharacter 0)))
      (bind _result (Math|Integer|IncrementInt (Variables|/Game/FirstPersonBP/Blueprints/FirstPersonCharacter.FirstPersonCharacter_C|GetPuzzlesComplete _asfirst_person_character))
        (:%20%20
          (Variables|/Game/FirstPersonBP/Blueprints/FirstPersonCharacter.FirstPersonCharacter_C|SetPuzzlesComplete _asfirst_person_character _result))))
    (else
      (Rendering|Material|SetMaterial (Variables|Default|GetHall_Wall_C1) 2 "/Game/StarterBundle/ModularScifiHallways/Materials/MI_Trims_B_2.MI_Trims_B_2")
      (Variables|Default|SetButtonCheck1 false)
      (Rendering|Material|SetMaterial (Variables|Default|GetHall_Wall_C2) 2 "/Game/StarterBundle/ModularScifiHallways/Materials/MI_Trims_B_2.MI_Trims_B_2")
      (Variables|Default|SetButtonCheck2 false)
      (Rendering|Material|SetMaterial (Variables|Default|GetHall_Wall_C3) 2 "/Game/StarterBundle/ModularScifiHallways/Materials/MI_Trims_B_2.MI_Trims_B_2")
      (Variables|Default|SetButtonCheck3 false))))

(event OnComponentBeginOverlap(TriggerSouth)
  (params (OverlappedComponent :type Primitive%20Component%20Object%20Reference) (OtherActor :type Actor%20Object%20Reference) (OtherComp :type Primitive%20Component%20Object%20Reference) (OtherBodyIndex :type Integer) (bFromSweep :type Boolean) (SweepResult :type Hit%20Result%20Structure%20%28by%20ref%29))
  ;[1 1 1] DoorAnimBack
  (if (Math|Boolean|ANDBoolean (stale OnComponentHit(HitCheck1) _output_get) (stale OnComponentHit(HitCheck2) _output_get) (stale OnComponentHit(HitCheck3) _output_get) (stale OnComponentHit(HitCheck4) _output_get))
    (Utilities|Casting|CastToFirstPersonCharacter OtherActor)
    (Variables|Default|SetDoorOpen false)
    (Audio|PlaySoundatLocation "/Game/Sounds/AirlockHiss.AirlockHiss" "0, 0, 0" "0, 0, 0" 1.0 1.0 0.0 0 0 0)
    (bind _dooranimunlock (Timeline|DoorAnimBack Play)
      (:Update
        (Transformation|SetRelativeLocation (Variables|Default|GetHall_Door_L) (Math|Vector|Lerp(Vector) "0, 0, 0" "0,-20.000000, 0" _dooranimunlock) false false))
      (:Finished
        (if (Math|Vector|Equal(Vector) (.Location (Math|Transform|BreakTransform (Transformation|GetRelativeTransform (Variables|Default|GetHall_Door_L)))) "0,-20.000000, 0" 1.0)
          ;[1 1 1] DoorAnimUp
          (Utilities|FlowControl|Delay 1.0)
          (Audio|PlaySoundatLocation "/Game/Sounds/AirlockDoorOpen.AirlockDoorOpen" "0, 0, 0" "0, 0, 0" 1.0 1.0 0.0 0 0 0)
          (bind _dooranimup (Timeline|DoorAnimUp Play)
            (:Update
              (Transformation|SetRelativeLocation (Variables|Default|GetHall_Door_L) (Math|Vector|Lerp(Vector) "0,-20.000000, 0" "0,-30.000000,400.000000" _dooranimup) false false))
            (:Finished
              (if (Variables|Default|GetDoorOpen)
                (Timeline|DoorAnimBack Reverse)
                (else
                  (Variables|Default|SetDoorOpen true))))))))))

(event OnComponentHit(HitCheck3)
  (params (HitComponent :type Primitive%20Component%20Object%20Reference) (OtherActor :type Actor%20Object%20Reference) (OtherComp :type Primitive%20Component%20Object%20Reference) (NormalImpulse :type Vector :default "0, 0, 0") (Hit :type Hit%20Result%20Structure%20%28by%20ref%29))
  ;[1 1 1] Button Check
  (bind _asfirst_person_projectile (Utilities|Casting|CastToFirstPersonProjectile OtherActor))
  (Actor|DestroyActor _asfirst_person_projectile)
  (if (and (Variables|Default|GetButtonCheck1) (Variables|Default|GetButtonCheck2))
    (Rendering|Material|SetMaterial (Variables|Default|GetHall_Wall_C3) 2 "/Game/Mayo_OriginalMaterials/M_GreenLight.M_GreenLight")
    (bind _output_get (Variables|Default|SetButtonCheck3 true))
    (else
      (Rendering|Material|SetMaterial (Variables|Default|GetHall_Wall_C1) 2 "/Game/StarterBundle/ModularScifiHallways/Materials/MI_Trims_B_2.MI_Trims_B_2")
      (Variables|Default|SetButtonCheck1 false)
      (Rendering|Material|SetMaterial (Variables|Default|GetHall_Wall_C2) 2 "/Game/StarterBundle/ModularScifiHallways/Materials/MI_Trims_B_2.MI_Trims_B_2")
      (Variables|Default|SetButtonCheck2 false))))

(event OnComponentHit(HitCheck2)
  (params (HitComponent :type Primitive%20Component%20Object%20Reference) (OtherActor :type Actor%20Object%20Reference) (OtherComp :type Primitive%20Component%20Object%20Reference) (NormalImpulse :type Vector :default "0, 0, 0") (Hit :type Hit%20Result%20Structure%20%28by%20ref%29))
  ;[1 1 1] Button Check
  (bind _asfirst_person_projectile (Utilities|Casting|CastToFirstPersonProjectile OtherActor))
  (Actor|DestroyActor _asfirst_person_projectile)
  (if (Variables|Default|GetButtonCheck1)
    (Rendering|Material|SetMaterial (Variables|Default|GetHall_Wall_C2) 2 "/Game/Mayo_OriginalMaterials/M_GreenLight.M_GreenLight")
    (bind _output_get (Variables|Default|SetButtonCheck2 true))
    (else
      (Rendering|Material|SetMaterial (Variables|Default|GetHall_Wall_C1) 2 "/Game/StarterBundle/ModularScifiHallways/Materials/MI_Trims_B_2.MI_Trims_B_2")
      (Variables|Default|SetButtonCheck1 false))))

(event OnComponentHit(HitCheck1)
  (params (HitComponent :type Primitive%20Component%20Object%20Reference) (OtherActor :type Actor%20Object%20Reference) (OtherComp :type Primitive%20Component%20Object%20Reference) (NormalImpulse :type Vector :default "0, 0, 0") (Hit :type Hit%20Result%20Structure%20%28by%20ref%29))
  ;[1 1 1] Button Check
  (bind _asfirst_person_projectile (Utilities|Casting|CastToFirstPersonProjectile OtherActor))
  (Actor|DestroyActor _asfirst_person_projectile)
  (Rendering|Material|SetMaterial (Variables|Default|GetHall_Wall_C1) 2 "/Game/Mayo_OriginalMaterials/M_GreenLight.M_GreenLight")
  (bind _output_get (Variables|Default|SetButtonCheck1 true)))

(fn ConstructionScript)

(fn EasyButtonPuzzle)